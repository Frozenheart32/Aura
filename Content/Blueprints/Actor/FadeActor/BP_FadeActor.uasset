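; BP_FadeActor is a mesh actor that fades out and back in by driving a "Fade" material parameter.
; The construction script creates dynamic instances of the mesh's materials, which BeginPlay applies to the mesh.
; FadeOut and Fadein play and reverse one timeline that updates every instance.
; With BlockVisibility set, BeginPlay blocks GameTraceChannel2, and FadeFinished sets Block for non-negative fade values, Ignore for negative ones.
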(event EventBeginPlay
  (CallFunction|SetMaterialstoDynamicInstances)
  (if (Variables|FadeSettings|GetBlockVisibility)
    (Collision|SetCollisionResponsetoChannel (Variables|Default|GetMesh) "ECC_GameTraceChannel2" "ECR_Block")))

(event EventFadein
  (bind _fade (Timeline|FadeTimeLine Reverse)
    (:Update
      (CallFunction|ChangeFadeMaterialValue _fade))
    (:Finished
      (CallFunction|FadeFinished _fade))))

(event EventFadeOut
  (bind _fade (Timeline|FadeTimeLine Play)
    (:Update
      (CallFunction|ChangeFadeMaterialValue _fade))
    (:Finished
      (CallFunction|FadeFinished _fade))))

(fn ConstructionScript
  (Utilities|Array|Clear (Variables|Default|GetDynamicMaterialInstancies))
  (bind _output_get (Variables|Default|SetOriginalMaterials (Rendering|Material|GetMaterials (Variables|Default|GetMesh))))
  (for _array_element _output_get
    (bind _returnvalue (Rendering|Material|CreateDynamicMaterialInstance _array_element "None" "None" :!class /Script/Engine.KismetMaterialLibrary))
    (Utilities|Array|AddUnique (Variables|Default|GetDynamicMaterialInstancies) _returnvalue)))

(fn SetMaterialstoDynamicInstances
  (for (_array_element _array_index) (Variables|Default|GetDynamicMaterialInstancies)
    (Rendering|Material|SetMaterial (Variables|Default|GetMesh) _array_index _array_element)))

(fn ChangeFadeMaterialValue
  (params (NewFadeValue :type Float%20%28double-precision%29))
  (for _array_element (Variables|Default|GetDynamicMaterialInstancies)
    (Rendering|Material|SetScalarParameterValue _array_element "Fade" NewFadeValue :!class /Script/Engine.MaterialInstanceDynamic)))

(fn FadeFinished
  (params (FadeValue :type Float%20%28double-precision%29))
  (bind _mesh (Variables|Default|GetMesh))
  (if (>= FadeValue 0.0)
    (if (Variables|FadeSettings|GetBlockVisibility)
      (Collision|SetCollisionResponsetoChannel _mesh "ECC_GameTraceChannel2" "ECR_Block"))
    (elif (<= FadeValue 0.0)
      (if (Variables|FadeSettings|GetBlockVisibility)
        (Collision|SetCollisionResponsetoChannel _mesh "ECC_GameTraceChannel2" "ECR_Ignore")))))