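; Enemy melee attack ability that turns the avatar toward its combat target and plays a randomly chosen tagged attack montage.
; The montage's gameplay event triggers a small sphere check at the matching combat socket, drawn as a debug sphere, damaging live non-friendly players inside.
; A hit fires the melee impact gameplay cue tagged with the montage tag.
; The ability ends after that event, or cancels without a valid target.
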(event Ability|EventActivateAbility
  (bind _returnvalue (Ability|GetAvatarActorfromActorInfo))
  (bind _returnvalue_2 (Ability|GetAvatarActorfromActorInfo))
  (bind _returnvalue_3 (Ability|GetAbilityLevel))
  (if (and (Utilities|DoesObjectImplementInterface _returnvalue "/Script/Aura.CombatInterface") (Utilities|DoesObjectImplementInterface _returnvalue "/Script/Aura.EnemyInterface"))
    (bind _returnvalue_4 (Class|EnemyInterface|GetCombatTarget(Message) _returnvalue))
    (Utilities|IsValid _returnvalue_4
      (:Is%20Valid
        (bind _output_get (Variables|Default|SetCombatTarget _returnvalue_4))
        (Class|CombatInterface|UpdateFacingTarget(Message) _returnvalue (Transformation|GetActorLocation _output_get))
        (bind _returnvalue_5 (Class|CombatInterface|GetAttackMontages(Message) (Ability|GetAvatarActorfromActorInfo)))
        (bind _output_get_2 (Variables|Default|SetSelectedTaggedMontage (Class|AuraDamageGameplayAbility|GetRandomTaggedMontagefromArray _returnvalue_5)))
        (|PlayMontageandWaitProxy "None" (.Montage (Utilities|Struct|BreakTaggedMontage _output_get_2)) 1.0 "None" false 1.0 0.0 false
          (:then
            (Ability|Tasks|WaitGameplayEvent (.MontageTag (Utilities|Struct|BreakTaggedMontage _output_get_2)) 0
              (:EventReceived
                (bind _returnvalue_6 (Class|CombatInterface|GetCombatSocketLocation(Message) (Ability|GetAvatarActorfromActorInfo) (.SocketTag (Utilities|Struct|BreakTaggedMontage (Variables|Default|GetSelectedTaggedMontage)))))
                (bind _output_get_3 (Variables|Default|SetCombatSocketLocation _returnvalue_6))
                (Rendering|Debug|DrawDebugSphere _output_get_3 45.0 12 "(R=1.000000,G=0.138097,B=0.000000,A=1.000000)" 0.5)
                (bind _outoverlappingactors (Class|AuraAbilitySystemLibrary|GetLivePlayerswithRadius _returnvalue_2 (Utilities|Array|MakeArray _returnvalue_2) 45.0 (Variables|Default|GetCombatSocketLocation)))
                (Variables|Default|SetHasHitTarget false)
                (for _array_element _outoverlappingactors
                  (if (Class|AuraAbilitySystemLibrary|IsNotFriend _array_element (Ability|GetAvatarActorfromActorInfo))
                    (Class|AuraDamageGameplayAbility|CauseDamage _array_element)
                    (Variables|Default|SetHasHitTarget true)))
                (if (Variables|Default|GetHasHitTarget)
                  (Class|GameplayAbility|ExecuteGameplayCuewithParams "(TagName=\"GameplayCue.MeleeImpact\")" (Ability|GameplayCue|MakeGameplayCueParameters :AggregatedSourceTags (GameplayTags|MakeGameplayTagContainerfromTag (.MontageTag (Utilities|Struct|BreakTaggedMontage (Variables|Default|GetSelectedTaggedMontage)))) :Location (Variables|Default|GetCombatSocketLocation) :EffectCauser (Ability|GetAvatarActorfromActorInfo) :SourceObject (Variables|Default|GetCombatTarget) :GameplayEffectLevel _returnvalue_3 :AbilityLevel _returnvalue_3)))
                (Ability|EndAbility))))
          (:OnCompleted
            (Ability|CancelAbility :!label _label))
          (:OnInterrupted
            (goto _label))
          (:OnCancelled
            (goto _label))))
      (:Is%20Not%20Valid
        (Ability|CancelAbility)))
    (else
      (Ability|CancelAbility))))

(event Ability|EventOnEndAbility
  (params (bWasCancelled :type Boolean)))