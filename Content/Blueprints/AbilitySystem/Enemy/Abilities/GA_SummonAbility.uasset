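; Enemy gameplay ability in which a shaman summons random minions at a set of spawn locations.
; On activation it shuffles the locations, plays a Niagara ground effect at each and starts the summon montage.
; The montage's gameplay event starts a delay-based loop that spawns minions one by one, facing the summoner, with debug spheres, then ends the ability.
; An interrupted or cancelled montage cancels the ability.
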(event Ability|EventActivateAbility
  (bind _output_get (Variables|Default|SetSpawnLocations (Class|AuraSummonAbility|GetSpawnLocations false)))
  (Utilities|Array|Shuffle _output_get)
  (for _array_element _output_get
    (Niagara|SpawnSystematLocation "/Game/Assets/Effects/Combat/NS_GroundSummon.NS_GroundSummon" _array_element))
  (|PlayMontageandWaitProxy "None" "/Game/Assets/Enemies/Shaman/Animations/AM_Shaman_Summon.AM_Shaman_Summon" 1.0 "None" false 1.0 0.0 false
    (:then
      (Ability|Tasks|WaitGameplayEvent "(TagName=\"Montage.Attack.1\")" 0
        (:EventReceived
          (if (< (Variables|Default|GetSpawnLocationIndex) (Utilities|Array|Length (Variables|Default|GetSpawnLocations))) :!label _label
            (Rendering|Debug|DrawDebugSphere (Utilities|Array|Get(acopy) (Variables|Default|GetSpawnLocations) (Variables|Default|GetSpawnLocationIndex)) 25.0 12 "(R=1.000000,G=1.000000,B=1.000000,A=1.000000)" 4.0)
            (Game|SpawnActorfromClass (Class|AuraSummonAbility|GetRandomMinionSubclass) (Math|Transform|MakeTransform (+ (Utilities|Array|Get(acopy) (Variables|Default|GetSpawnLocations) (Variables|Default|GetSpawnLocationIndex)) "0.000000,0.000000,70.000000") (Math|Rotator|FindLookatRotation (+ (Utilities|Array|Get(acopy) (Variables|Default|GetSpawnLocations) (Variables|Default|GetSpawnLocationIndex)) "0.000000,0.000000,70.000000") (Transformation|GetActorLocation (Ability|GetAvatarActorfromActorInfo))) "1.000000,1.000000,1.000000") "AdjustIfPossibleButAlwaysSpawn" "MultiplyWithRoot" 0 0)
            (Math|Integer|IncrementInt (Variables|Default|GetSpawnLocationIndex)
              (:%20%20
                (Utilities|FlowControl|Delay 0.2)
                (goto _label)))
            (else
              (Ability|EndAbility))))))
    (:OnInterrupted
      (Ability|CancelAbility :!label _label_2))
    (:OnCancelled
      (goto _label_2))))

(event Ability|EventOnEndAbility
  (params (bWasCancelled :type Boolean)))