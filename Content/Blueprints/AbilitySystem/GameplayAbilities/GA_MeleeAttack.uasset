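; GA_MeleeAttack is a gameplay ability for an enemy melee attack on its combat target.
; It turns the avatar toward the target via combat and enemy interfaces and plays a random tagged attack montage.
; When the montage's tag event fires, it damages live players within a small debug-drawn sphere at that tag's combat socket, then ends.
; Missing interfaces, target or montages cancel it, as does the montage completing or being interrupted.
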(event Ability|EventActivateAbility
  (bind _returnvalue (Ability|GetAvatarActorfromActorInfo))
  (bind _returnvalue_2 (Ability|GetAvatarActorfromActorInfo))
  (if (and (Utilities|DoesObjectImplementInterface _returnvalue_2 "/Script/Aura.CombatInterface") (Utilities|DoesObjectImplementInterface _returnvalue_2 "/Script/Aura.EnemyInterface"))
    (bind _returnvalue_3 (Class|EnemyInterface|GetCombatTarget(Message) _returnvalue_2))
    (Utilities|IsValid _returnvalue_3
      (:Is%20Valid
        (Class|CombatInterface|UpdateFacingTarget(Message) _returnvalue_2 (Transformation|GetActorLocation _returnvalue_3))
        (bind _returnvalue_4 (Class|CombatInterface|GetAttackMontages(Message) (Ability|GetAvatarActorfromActorInfo)))
        (if (> (Utilities|Array|Length _returnvalue_4) 0)
          (bind _output_get (Variables|Default|SetSelectedTaggedMontage (Utilities|Array|Get(acopy) _returnvalue_4 (Math|Random|RandomIntegerinRange 0 (- (Utilities|Array|Length _returnvalue_4) 1)))))
          (|PlayMontageandWaitProxy "None" (.Montage (Utilities|Struct|BreakTaggedMontage _output_get)) 1.0 "None" false 1.0 0.0 false
            (:then
              (Ability|Tasks|WaitGameplayEvent (.MontageTag (Utilities|Struct|BreakTaggedMontage _output_get)) 0
                (:EventReceived
                  (bind _returnvalue_5 (Class|CombatInterface|GetCombatSocketLocation(Message) (Ability|GetAvatarActorfromActorInfo) (.MontageTag (Utilities|Struct|BreakTaggedMontage _output_get))))
                  (Rendering|Debug|DrawDebugSphere _returnvalue_5 45.0 12 "(R=1.000000,G=0.138097,B=0.000000,A=1.000000)" 0.5)
                  (bind _outoverlappingactors (Class|AuraAbilitySystemLibrary|GetLivePlayerswithRadius _returnvalue (Utilities|Array|MakeArray _returnvalue) 45.0 _returnvalue_5))
                  (for _array_element _outoverlappingactors
                    (Class|AuraDamageGameplayAbility|CauseDamage _array_element))
                  (Ability|EndAbility))))
            (:OnCompleted
              (Ability|CancelAbility :!label _label))
            (:OnInterrupted
              (goto _label))
            (:OnCancelled
              (goto _label)))
          (else
            (Ability|CancelAbility))))
      (:Is%20Not%20Valid
        (Ability|CancelAbility)))
    (else
      (Ability|CancelAbility))))

(event Ability|EventOnEndAbility
  (params (bWasCancelled :type Boolean)))