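; GA_Firebolt is the Fire ability that casts homing Firebolt projectiles at the target under the mouse.
; After committing, it takes cursor target data, turns the avatar via CombatInterface and plays the cast montage.
; The non-authority side waits for the montage event while authority goes straight to a BothWait net sync.
; On sync, it spawns pitched projectiles from the weapon socket, homing on the hit actor, then ends.
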(event Ability|EventActivateAbility
  (bind _returnvalue (Ability|CommitAbility))
  (if _returnvalue
    (bind _data (|TargetDataUnderMouse)
      (:ValidData
        (Variables|Default|SetProjectileTargetLocation (.Location (Collision|BreakHitResult (Ability|TargetData|GetHitResultfromTargetData _data))))
        (Variables|Default|SetMouseHitActor (.HitActor (Collision|BreakHitResult (Ability|TargetData|GetHitResultfromTargetData _data))))
        (bind _ascombat_interface (Utilities|Casting|CastToCombatInterface (Ability|GetAvatarActorfromActorInfo))
          (:then
            (Class|CombatInterface|UpdateFacingTarget _ascombat_interface (Variables|Default|GetProjectileTargetLocation))
            (|PlayMontageandWaitProxy "None" "/Game/Assets/Characters/Aura/Animations/Abilities/AM_Cast_FireBolt.AM_Cast_FireBolt" 1.0 "None" false 1.0 0.0 false
              (:then
                (Ability|HasAuthority
                  (:True
                    _)
                  (:False
                    (Ability|Tasks|WaitGameplayEvent "(TagName=\"Event.Montage.Firebolt\")" 0
                      (:EventReceived
                        _))))
                (Ability|Tasks|WaitNetSync "BothWait"
                  (:OnSync
                    (Class|AuraFireBolt|SpawnProjectiles (Variables|Default|GetProjectileTargetLocation) (GameplayTags|MakeLiteralGameplayTag "(TagName=\"CombatSocket.Weapon\")") true 55.0 (Variables|Default|GetMouseHitActor))
                    (Ability|EndAbility))))))
          (:CastFailed
            (Ability|CancelAbility)))))
    (else
      (Ability|CancelAbility))))

(event Ability|EventOnEndAbility
  (params (bWasCancelled :type Boolean)))