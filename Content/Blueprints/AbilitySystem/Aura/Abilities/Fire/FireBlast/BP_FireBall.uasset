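; BP_FireBall is a boomerang-style fireball projectile that flies outward, then returns to a target actor and explodes.
; StartOutgoingTimeline runs only on the server, lerping the ball along its forward vector to an apex at TravelDistance.
; A second timeline then lerps it toward ReturnToActor's live location, so it tracks movement.
; Once within ExplodeDistance of that actor, it calls OnHit and destroys itself.
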(event EventStartOutgoingTimeline
  (bind _returntoactor (Variables|Default|GetReturnToActor))
  (Networking|SwitchHasAuthority
    (:Authority
      (Variables|Default|SetInitialLocation (Transformation|GetActorLocation))
      (Variables|Default|SetApexLocation (+ (Variables|Default|GetInitialLocation) (* (Transformation|GetActorForwardVector) (Variables|Default|GetTravelDistance))))
      (bind _outgoingtrack (Timeline|OutgoingTimeline Play)
        (:Update
          (Transformation|SetActorLocation (Math|Vector|Lerp(Vector) (Variables|Default|GetInitialLocation) (Variables|Default|GetApexLocation) _outgoingtrack) false false))
        (:Finished
          (bind _returningtrack (Timeline|ReturningTimeline Play)
            (:Update
              (Utilities|IsValid _returntoactor
                (:Is%20Valid
                  (Transformation|SetActorLocation (Math|Vector|Lerp(Vector) (Variables|Default|GetApexLocation) (Transformation|GetActorLocation _returntoactor) _returningtrack) false false)
                  (if (CallFunction|IsWithinExplodeDistance)
                    (Class|AuraProjectile|OnHit)
                    (Actor|DestroyActor)))))))))))

(fn ConstructionScript)

(fn IsWithinExplodeDistance
  (return (<= (Math|Vector|VectorLength (- (Transformation|GetActorLocation) (Transformation|GetActorLocation (Variables|Default|GetReturnToActor)))) (Variables|Default|GetExplodeDistance))))